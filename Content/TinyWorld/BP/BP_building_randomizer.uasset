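; City building randomizer that extends a parent generator, decorating instanced buildings with rooftop and wall holograms.
; After each building is created, it probability-tests numbered "holo_rooftop_" and "holo_wall_" mesh sockets and stores hologram data with random material indices.
; RefreshHolos rebuilds holograms from that data after CreateMeshes, as billboard child actors and static mesh components placed from socket and instance transforms.
; Older construction-script randomization remains as disconnected logic.
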(fn ConstructionScript
  (|CallParentFunction))

(fn SetRooftopHologram
  (params (component :type Child%20Actor%20Component%20Object%20Reference) (index :type Integer))
  (bind _asbp_holo_billboard (Utilities|Casting|CastToBP_Holo_Billboard (Variables|/Script/Engine.ChildActorComponent|GetChildActor component)))
  (Default|SetMaterial _asbp_holo_billboard (Utilities|Array|Get(acopy) (Variables|Editablevariables|GetRooftopHoloMaterials) index)))

(fn SetWallHologram
  (params (Component :type Static%20Mesh%20Component%20Object%20Reference) (Index :type Integer))
  (Rendering|Material|SetMaterial Component 0 (Utilities|Array|Get(acopy) (Variables|Editablevariables|GetWallHoloMaterials) Index)))

(fn OnPostBuildingCreated
  (params (BuildingRef :type City%20Building%20Structure%20%28by%20ref%29))
  (bind (_location _size _offsetindex _rotationindex _scaleindex _meshindex _meshinstanceid) (Utilities|Struct|BreakCityBuilding BuildingRef))
  (LocalVariables|SetMeshInstanceIndex _meshinstanceid)
  (bind _output_get (LocalVariables|SetMeshTypeIndex _meshindex))
  (LocalVariables|SetMesh (Utilities|Array|Get(acopy) (Variables|Default|GetBuildingMeshes) _output_get))
  (Utilities|FlowControl|Sequence
    (:then_0
      ;[1 0.8438 0] Add holo on rooftop
      (while (Utilities|IsValid (Class|StaticMesh|FindSocket (LocalVariables|GetMesh) (Utilities|String|StringToName (Utilities|String|Append "holo_rooftop_" (Utilities|String|ToString(Integer) (LocalVariables|GetIndex))))))
        (if (< (Math|Random|RandomFloatinRange 0.0 1.0) (Variables|EditableVariables|GetRooftopProbability))
          (Utilities|Array|Add (Variables|Default|GetRooftopHoloDatas) (Utilities|Struct|MakeHoloData (LocalVariables|GetMeshTypeIndex) (LocalVariables|GetMeshInstanceIndex) (Math|Random|RandomIntegerinRange 0 (- (Utilities|Array|Length (Variables|Editablevariables|GetRooftopHoloMaterials)) 1)) (Utilities|String|StringToName (Utilities|String|Append "holo_rooftop_" (Utilities|String|ToString(Integer) (LocalVariables|GetIndex))))))
          (CallFunction|SpawnRooftopHolo (Utilities|Struct|MakeHoloData (LocalVariables|GetMeshTypeIndex) (LocalVariables|GetMeshInstanceIndex) (Math|Random|RandomIntegerinRange 0 (- (Utilities|Array|Length (Variables|Editablevariables|GetRooftopHoloMaterials)) 1)) (Utilities|String|StringToName (Utilities|String|Append "holo_rooftop_" (Utilities|String|ToString(Integer) (LocalVariables|GetIndex)))))))
        (Math|Integer|IncrementInt (LocalVariables|GetIndex))))
    (:then_1
      (LocalVariables|SetIndex 0)
      (while (Utilities|IsValid (Class|StaticMesh|FindSocket (LocalVariables|GetMesh) (Utilities|String|StringToName (Utilities|String|Append "holo_wall_" (Utilities|String|ToString(Integer) (LocalVariables|GetIndex))))))
        (if (< (Math|Random|RandomFloatinRange 0.0 1.0) (Variables|EditableVariables|GetWallProbability))
          (Utilities|Array|Add (Variables|Default|GetWallHoloDatas) (Utilities|Struct|MakeHoloData (LocalVariables|GetMeshTypeIndex) (LocalVariables|GetMeshInstanceIndex) (Math|Random|RandomIntegerinRange 0 (- (Utilities|Array|Length (Variables|Editablevariables|GetWallHoloMaterials)) 1)) (Utilities|String|StringToName (Utilities|String|Append "holo_wall_" (Utilities|String|ToString(Integer) (LocalVariables|GetIndex)))))))
        (Math|Integer|IncrementInt (LocalVariables|GetIndex))))))

(fn UpdateValues
  (Variables|Default|SetCitySize (Math|Vector2D|MakeVector2D (Math|Conversions|ToFloat(Integer) (Variables|Editablevariables|GetRows)) (Math|Conversions|ToFloat(Integer) (Variables|Editablevariables|Getcolumns)))))

(fn ClearCity
  (|CallParentFunction)
  (Utilities|Array|Clear (Variables|Default|GetWallHoloDatas))
  (Utilities|Array|Clear (Variables|Default|GetRooftopHoloDatas))
  (CitySetup|ClearHolosMeshes))

(fn SpawnRooftopHolo
  (params (HoloData :type Holo%20Data%20Structure%20%28by%20ref%29))
  (bind (_meshindex _meshinstanceindex _holoindex _socketname) (Utilities|Struct|BreakHoloData HoloData))
  (bind _buildingmeshescomponent (Variables|Default|GetBuildingMeshesComponent))
  (bind _output (Utilities|Array|Get(acopy) _buildingmeshescomponent _meshindex))
  (bind _outinstancetransform (Components|InstancedStaticMesh|GetInstanceTransform _output _meshinstanceindex false))
  (bind _returnvalue (AddComponent|AddChildActorComponent false (Math|Transform|MakeTransform (+ (* (Variables|/Script/Engine.StaticMeshSocket|GetRelativeLocation (Class|StaticMesh|FindSocket (Utilities|Array|Get(acopy) (Variables|Default|GetBuildingMeshes) _meshindex) _socketname)) (.scale _outinstancetransform)) (.location _outinstancetransform)) "0, 0, 0" "1,1,1")))
  (Utilities|Array|Add (Variables|arrays|Getspawned%20RooftopHolograms) _returnvalue)
  (CallFunction|SetRooftopHologram _returnvalue _holoindex))

(fn SpawnWallHolo
  (params (HoloData :type Holo%20Data%20Structure%20%28by%20ref%29))
  (bind (_meshindex _meshinstanceindex _holoindex _socketname) (Utilities|Struct|BreakHoloData HoloData))
  (bind _buildingmeshes (Variables|Default|GetBuildingMeshes))
  (bind _buildingmeshescomponent (Variables|Default|GetBuildingMeshesComponent))
  (bind _output (Utilities|Array|Get(acopy) _buildingmeshes _meshindex))
  (bind _output_2 (Utilities|Array|Get(acopy) _buildingmeshescomponent _meshindex))
  (bind _returnvalue (Class|StaticMesh|FindSocket _output _socketname))
  (bind _outinstancetransform (Components|InstancedStaticMesh|GetInstanceTransform _output_2 _meshinstanceindex false))
  (bind _returnvalue_2 (AddComponent|AddStaticMeshComponent false (Math|Transform|MakeTransform (+ (* (Variables|/Script/Engine.StaticMeshSocket|GetRelativeLocation _returnvalue) (.scale _outinstancetransform)) (.location _outinstancetransform)) (Variables|/Script/Engine.StaticMeshSocket|GetRelativeRotation _returnvalue) (* (.scale _outinstancetransform) (Variables|EditableVariables|GetHoloWallsScale)))))
  (Utilities|Array|Add (Variables|arrays|Getspawned%20WallHolograms) _returnvalue_2)
  (CallFunction|SetWallHologram _returnvalue_2 _holoindex))

(fn CreateMeshes
  (|CallParentFunction)
  (CitySetup|RefreshHolos))

(fn RefreshHolos
  (CitySetup|ClearHolosMeshes)
  (for _array_element (Variables|Default|GetRooftopHoloDatas)
    (CallFunction|SpawnRooftopHolo _array_element))
  (for _array_element_2 (Variables|Default|GetWallHoloDatas)
    (CallFunction|SpawnWallHolo _array_element_2)))

(fn ClearHolosMeshes
  (bind _spawned_wallholograms (Variables|arrays|Getspawned%20WallHolograms))
  (bind _spawned_rooftopholograms (Variables|arrays|Getspawned%20RooftopHolograms))
  (for _array_element _spawned_rooftopholograms
    (Utilities|IsValid _array_element
      (:Is%20Valid
        (Components|DestroyComponent _array_element))))
  (Utilities|Array|Clear _spawned_rooftopholograms)
  (for _array_element_2 _spawned_wallholograms
    (Utilities|IsValid _array_element_2
      (:Is%20Valid
        (Components|DestroyComponent _array_element_2))))
  (Utilities|Array|Clear _spawned_wallholograms))